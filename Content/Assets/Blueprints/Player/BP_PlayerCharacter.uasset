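; Player character Blueprint that adds camera and audio feedback for movement and looking, plus the flashlight toggle.
; Tick gates footstep and wobble timelines on speed, with sprinting increasing footstep frequency and punch scale.
; Footsteps line-trace downward to choose sounds by surface type, with a harsher variant when sprinting.
; Look input scales a turn shake and feeds a smoothed parameter into a looping MetaSound camera-turn swoosh.
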(event `self.ReceiveBeginPlay`
  ;[1 1 1] Setup
  (`|ExecutionSequence`
    (:`then_0`
      (bind _asbp_player_controller (cast `/Game/Assets/Blueprints/Player/BP_PlayerController` (`GameplayStatics.GetPlayerController` 0)))
      (set `self.As BP Player Controller` _asbp_player_controller))
    (:`then_3`
      (`|ExecutionSequence`
        (:`then_0`
          (bind _returnvalue (`GameplayStatics.SpawnSound2D` "/Game/Assets/Audio/SFX/Player/Camera/MS_CameraTurn.MS_CameraTurn" 0.8 1.0 0.0 null))
          (bind _output_get (set `self.Camera Turn Sound` _returnvalue))
          (`AudioComponent.Play` _output_get 0.0)
          (`CameraShakeSourceComponent.StartCameraShake` :`self` (`self.Camera Wobble`)))
        (:`then_1`
          (`CameraShakeSourceComponent.StartCameraShake` :`self` (`self.Camera Wobble`)))))))

(event `EnhancedInput|/Game/Assets/Blueprints/Player/Input/IA_Flashlight`
  (params (ActionValue :type Boolean) (ElapsedSeconds :type "Float (double-precision)") (TriggeredSeconds :type "Float (double-precision)") (InputAction :type "InputAction Object Reference" :default "/Game/Assets/Blueprints/Player/Input/IA_Flashlight.IA_Flashlight"))
  ;[1 1 1] Flashlight toggle (TODO: move to C++)
  (:`Started`
    (`FlashlightComponent.ToggleFlashlight` (`self.Flashlight`))))

(event `self.ReceiveTick`
  (params (DeltaSeconds :type "Float (single-precision)"))
  (bind _bissprinting (`self.bIsSprinting`))
  ;[1 1 1] Camera shake
  (set `self.Delta Seconds` DeltaSeconds)
  (`|ExecutionSequence`
    (:`then_0`
      ;;[1 1 1] Camera bob
      (bind _reference (`self.UpdatePlayerVelocity`))
      (`|ExecutionSequence`
        (:`then_0`
          (bind _returnvalue (> _reference 50.0))
          (if _returnvalue
            (`Timeline|Footstep Timeline` :!label _label
              (:`Trigger`
                (`/Engine/EditorBlueprintResources/StandardMacros.FlipFlop`
                  (:`A`
                    (`CameraShakeSourceComponent.StartCameraShake` :`self` (`self.Camera Punch`) :`InCameraShake` "/Game/Assets/Other/PostProcessing/CameraShake/CSB_Footstep.CSB_Footstep_C" :`Scale` (`KismetMathLibrary.SelectFloat` 1.8 1.0 _bissprinting) :!label _label_2)
                    (`self.Play Footstep Sound`))
                  (:`B`
                    (if _bissprinting
                      (goto _label_2))))))
            (else
              (`|ExecutionSequence`
                (:`then_0`
                  (goto _label :!via `SetNewTime`))
                (:`then_1`
                  (goto _label :!via `Stop`))))))
        (:`then_1`
          (if _returnvalue
            (`Timeline|Wobble` :!label _label_3
              (:`Wobble`
                (`self.PlayCorrespondingWobble` _returnvalue)))
            (else
              (goto _label_3 :!via `Stop`))))))
    (:`then_1`
      ;;[1 1 1] Audio swoosh when turning
      (bind _output_get (set `self.Audio Camera Turn` (`KismetMathLibrary.Lerp` (`self.Audio Camera Turn`) (`self.Audio Camera Turn Target`) (* (`self.Delta Seconds`) 5.0))))
      (`AudioParameterControllerInterface.SetFloatParameter` (`self.Camera Turn Sound`) "Travel speed" (* _output_get 0.3)))))

(event `EnhancedInput|/Game/Assets/Blueprints/Player/Input/IA_Look`
  (params (ActionValue :type "Vector2D Structure") (ElapsedSeconds :type "Float (double-precision)") (TriggeredSeconds :type "Float (double-precision)") (InputAction :type "InputAction Object Reference" :default "/Game/Assets/Blueprints/Player/Input/IA_Look.IA_Look"))
  (bind _returnvalue (* (`KismetMathLibrary.VSize2D` ActionValue) 0.5))
  ;[1 1 1] Head turn wobble
  (:`Triggered`
    (set `self.Audio Camera Turn Target` _returnvalue)
    (`CameraShakeSourceComponent.StartCameraShake` :`self` (`self.Camera Turn Wobble`) :`Scale` _returnvalue)))

(fn `Play Footstep Sound`
  (bind _footsteps (`self.Footsteps`))
  (bind _footsteps_2 (`self.Footsteps`))
  (bind _returnvalue (`SceneComponent.K2_GetComponentLocation` (`self.Footsteps`)))
  (bind _outhit (`KismetSystemLibrary.LineTraceSingle` _returnvalue (- _returnvalue (0.0 0.0 150.0)) "TraceTypeQuery1"))
  (`|ExecutionSequence`
    (:`then_0`
      (bind (_value _returnvalue_2) (`BlueprintMapLibrary.Map_Find` (`self.Footstep Sounds`) (`GameplayStatics.GetSurfaceType` _outhit)))
      ;[1 1 1] Audio based on stepped material
      (if _returnvalue_2
        (`AudioComponent.SetSound` _footsteps_2 _value)
        (else
          (`AudioComponent.SetSound` _footsteps_2 "/Game/Assets/Audio/SFX/Player/Footsteps/Default/MS_FootstepDefault.MS_FootstepDefault"))))
    (:`then_1`
      ;[1 1 1] Sprint loudness
      (`AudioParameterControllerInterface.SetBoolParameter` _footsteps "Harsh" (`self.bIsSprinting`)))
    (:`then_2`
      (`AudioComponent.Play` _footsteps 0.0))))

(fn `UpdatePlayerVelocity`
  (returns (Reference :type "Float (double-precision)"))
  (bind _output_get (set `self.Velocity` (`KismetMathLibrary.VSize` (`CharacterMovementComponent.GetLastUpdateVelocity` (`self.CharacterMovement`)))))
  (return _output_get))

(fn `UserConstructionScript`)